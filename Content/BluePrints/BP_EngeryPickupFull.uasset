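; BP_EngeryPickupFull is an energy pickup actor that refills the player robot's energy.
; On BeginPlay it caches the player character cast to BP_Robot.
; When the player overlaps its sphere component, it calls IncreaseEnergy on the robot with a full 100-point amount, then destroys itself.
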(event `self.ReceiveBeginPlay`
  (bind _asbp_robot (cast `/Game/LiamFolder/BP_Robot` (`GameplayStatics.GetPlayerCharacter` 0)))
  (`/Engine/EditorBlueprintResources/StandardMacros.IsValid` _asbp_robot
    (:`Is Valid`
      (set `self.Player` _asbp_robot))))

(event `self.Sphere.OnComponentBeginOverlap`
  (params (OverlappedComponent :type "PrimitiveComponent Object Reference") (OtherActor :type "Actor Object Reference") (OtherComp :type "PrimitiveComponent Object Reference") (OtherBodyIndex :type Integer) (bFromSweep :type Boolean) (SweepResult :type "HitResult Structure (by ref)"))
  (if (== OtherActor (`GameplayStatics.GetPlayerCharacter` 0))
    (`/Game/LiamFolder/BP_Robot.IncreaseEnergy` (`self.Player`) 100.0)
    (`self.K2_DestroyActor`)))

(fn `UserConstructionScript`)