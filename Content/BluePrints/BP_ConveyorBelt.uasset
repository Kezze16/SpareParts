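; BP_ConveyorBelt is a conveyor belt actor that carries whatever actors overlap its Box.
; Each Tick it offsets those actors along the StaticMesh's forward vector by Speed scaled by delta time, without sweeping.
; BeginPlay caches the player BP_Robot's Sphere, and Tick compares each overlapping actor against that reference to skip a match.
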(event `self.ReceiveBeginPlay`
  (bind _asbp_robot (cast `/Game/LiamFolder/BP_Robot` (`GameplayStatics.GetPlayerCharacter` 0)))
  (`/Engine/EditorBlueprintResources/StandardMacros.IsValid` _asbp_robot
    (:`Is Valid`
      (set `self.Sphere` (`/Game/LiamFolder/BP_Robot.Sphere` _asbp_robot)))))

(event `self.ReceiveTick`
  (params (DeltaSeconds :type "Float (single-precision)"))
  (for _array_element (`PrimitiveComponent.GetOverlappingActors` (`self.Box`) null)
    (if (!= _array_element (`self.Sphere`))
      (`self.K2_AddActorWorldOffset` _array_element (* (* DeltaSeconds (`self.Speed`)) (`KismetMathLibrary.GetForwardVector` (`SceneComponent.K2_GetComponentRotation` (`self.StaticMesh`)))) false false))))

(fn `UserConstructionScript`)